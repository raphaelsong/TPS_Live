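; Base character Blueprint that provides health, damage reaction, stun and defeat handling.
; CurrentHealth starts at MaxHealth on BeginPlay, and ReceiveAttack subtracts incoming damage from it.
; Surviving a hit sets IsStunned and starts a short timer, with ClearStun resetting the flag, while reaching zero health disables capsule collision.
; Both outcomes drive animation by jumping directly to named nodes in the Locomotion state machine.
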(event EventBeginPlay
  (Variables|Default|SetCurrentHealth (Variables|Default|GetMaxHealth)))

(event Collision|EventActorBeginOverlap
  (params (OtherActor :type Actor%20Object%20Reference)))

(event EventTick
  (params (DeltaSeconds :type Float%20%28single-precision%29)))

(fn ConstructionScript)

(fn ReceiveAttack
  (params (InDamage :type Float%20%28double-precision%29))
  (bind _output_get (Variables|Default|SetCurrentHealth (- (Variables|Default|GetCurrentHealth) InDamage)))
  (if (<= _output_get 0.0)
    (Class|PaperZDAnimInstance|JumptoNode (Class|PaperZDCharacter|GetAnimInstance) "JumpDefeated" "Locomotion")
    (Collision|SetCollisionEnabled (Variables|Default|GetCapsuleComponent) "NoCollision")
    (else
      (Variables|Default|SetIsStunned true)
      (Class|PaperZDAnimInstance|JumptoNode (Class|PaperZDCharacter|GetAnimInstance) "JumpStunned" "Locomotion")
      (Utilities|Time|SetTimerbyEvent (EventDispatchers|CreateEvent :!event ClearStun) 0.5))))

(fn ClearStun
  (Variables|Default|SetIsStunned false))