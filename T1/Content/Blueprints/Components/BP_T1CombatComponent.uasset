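; BP_T1CombatComponent is a combat component that tracks an actor's hit points and handles dealing and receiving damage.
; HP starts at its maximum on BeginPlay.
; CombatAttack looks up the same component on the hit actor and calls CombatHit, which subtracts damage, clamps the result and calls OnChangedHp, plus OnHpZero when HP reaches zero.
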(event EventBeginPlay
  (Variables|Default|SetHp (Variables|Default|GetMaxHp)))

(event EventTick
  (params (DeltaSeconds :type Float%20%28single-precision%29)))

(fn CombatAttack
  (params (InDamage :type Float%20%28double-precision%29) (HitActor :type Actor%20Object%20Reference))
  (bind _returnvalue (Actor|GetComponentbyClass HitActor "BP_T1CombatComponent_C"))
  (Utilities|IsValid _returnvalue
    (:Is%20Valid
      (CallFunction|CombatHit _returnvalue InDamage))))

(fn CombatHit
  (params (InDamage :type Float%20%28double-precision%29))
  (Variables|Default|SetHp (Math|Float|Clamp(Float) (- (Variables|Default|GetHp) InDamage) 0.0 (Variables|Default|GetMaxHp)))
  (Default|CallOnChangedHp (Variables|Default|GetHp) (Variables|Default|GetMaxHp))
  (if (<= (Variables|Default|GetHp) 0.0)
    (Default|CallOnHpZero)))