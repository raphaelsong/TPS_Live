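; Player controller that lets the player switch control between the BP_T1Character pawns in the level.
; On BeginPlay it caches every BP_T1Character actor in an array.
; Pressing the 1 key increments an index, wraps it by the array length with modulo, then unpossesses the current pawn and possesses the character at that index if valid.
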(event EventBeginPlay
  (bind _outactors (Actor|GetAllActorsOfClass "/Game/Blueprints/Character/BP_T1Character.BP_T1Character_C"))
  (Variables|Default|SetT1Characters _outactors))

(event EventTick
  (params (DeltaSeconds :type Float%20%28single-precision%29)))

(event Input|KeyboardEvents|1
  (params (Key :type Key%20Structure :default "None"))
  (:Pressed
    (bind _result (Math|Integer|IncrementInt (Variables|Default|GetNowIndex))
      (:%20%20
        (CallFunction|PossessT1Character (Math|Integer|%(Integer) _result (Utilities|Array|Length (Variables|Default|GetT1Characters))))))))

(fn ConstructionScript)

(fn PossessT1Character
  (params (NewIndex :type Integer))
  (if (Utilities|Array|IsValidIndex (Variables|Default|GetT1Characters) NewIndex)
    (Pawn|UnPossess)
    (Pawn|Possess (Utilities|Array|Get(acopy) (Variables|Default|GetT1Characters) NewIndex))))