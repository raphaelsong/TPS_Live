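; BP_T1Monster is a monster character with a melee attack, a widget HP bar and a death sequence.
; CombatComponent HP changes update the bar, and it also exposes an HP-zero binding.
; Attack sets an AnimBP flag and freezes movement until a one-second timer, while AttackHitCheck sphere-traces forward, with debug drawing, to deal damage.
; SetDead plays the death montage, hides the bar, disables collision, stops the AI controller and starts a delayed timer.
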(event Custom|UpdateHp
  (params (NewHp :type Float%20%28double-precision%29) (NewMaxHp :type Float%20%28double-precision%29))
  (bind _aswbp_hp_bar (Utilities|Casting|CastToWBP_HpBar (UserInterface|GetWidget (Variables|Default|GetHpBarWidgetComponent))))
  (Default|UpdateHp _aswbp_hp_bar NewHp NewMaxHp))

(event EventBeginPlay
  (bind _combatcomponent (Variables|Default|GetCombatComponent))
  (EventDispatchers|BindEventtoOnChangedHp (Variables|Default|GetCombatComponent) (delegate Custom|UpdateHp))
  (Default|CallOnChangedHp _combatcomponent (Variables|/Game/Blueprints/Components/BP_T1CombatComponent.BP_T1CombatComponent_C|GetHp _combatcomponent) (Variables|/Game/Blueprints/Components/BP_T1CombatComponent.BP_T1CombatComponent_C|GetMaxHp _combatcomponent))
  (EventDispatchers|BindEventtoOnHpZero (Variables|Default|GetCombatComponent) (EventDispatchers|CreateEvent :!event SetDead)))

(event Collision|EventActorBeginOverlap
  (params (OtherActor :type Actor%20Object%20Reference)))

(event EventTick
  (params (DeltaSeconds :type Float%20%28single-precision%29)))

(fn ConstructionScript)

(fn Attack
  (bind _asabp_t1monster (Utilities|Casting|CastToABP_T1Monster (Components|SkeletalMesh|GetAnimInstance (Variables|Character|GetMesh))))
  (Variables|/Game/Animation/Monster/ABP_T1Monster.ABP_T1Monster_C|SetAttack _asabp_t1monster true)
  (Pawn|Components|CharacterMovement|SetMovementMode (Variables|Character|GetCharacterMovement) "MOVE_None" 0)
  (Utilities|Time|SetTimerbyFunctionName 0 "AttackEnded" 1.0))

(fn AttackHitCheck
  (bind _returnvalue (Transformation|GetActorLocation))
  (bind (_outhit _returnvalue_2) (Collision|SphereTraceByChannel _returnvalue (+ _returnvalue (* (Transformation|GetActorForwardVector) (Variables|Default|GetAttackRange))) (Variables|Default|GetAttackRadius) "TraceTypeQuery4" false 0 "ForDuration" true "(R=1.000000,G=0.000000,B=0.000000,A=1.000000)" "(R=0.000000,G=1.000000,B=0.000000,A=1.000000)" 1.0))
  (if _returnvalue_2
    (Default|CombatAttack (Variables|Default|GetCombatComponent) (Variables|Default|GetAttackDamage) (.HitActor (Collision|BreakHitResult _outhit)))))

(fn AttackEnded
  (bind _asabp_t1monster (Utilities|Casting|CastToABP_T1Monster (Components|SkeletalMesh|GetAnimInstance (Variables|Character|GetMesh))))
  (Variables|/Game/Animation/Monster/ABP_T1Monster.ABP_T1Monster_C|SetAttack _asabp_t1monster false)
  (Pawn|Components|CharacterMovement|SetMovementMode (Variables|Character|GetCharacterMovement) "MOVE_Walking" 0))

(fn SetDead
  (Animation|PlayAnimMontage "/Game/Animation/Monster/AM_MonsterDeath.AM_MonsterDeath" 1.0 "None")
  (Development|SetHiddeninGame (Variables|Default|GetHpBarWidgetComponent) true false)
  (Collision|SetActorEnableCollision false)
  (Utilities|Time|SetTimerbyEvent (EventDispatchers|CreateEvent :!event K2DestroyActor) 5.0)
  (bind _asbp_t1monster_aicontroller (Utilities|Casting|CastToBP_T1MonsterAIController (Pawn|GetController)))
  (Default|StopAI _asbp_t1monster_aicontroller))