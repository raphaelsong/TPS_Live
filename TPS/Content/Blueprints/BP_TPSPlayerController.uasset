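; Player controller that lets the player cycle control through the pawns in the level with the 1 key.
; BeginPlay caches every Pawn actor into an array once.
; Each key press calls ChangePawn, which unpossesses the current pawn and possesses the one at the stored index if valid.
; The index then increments and wraps by the array length.
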(event EventBeginPlay
  (bind _outactors (Actor|GetAllActorsOfClass "/Script/Engine.Pawn"))
  (Variables|Default|SetOut%20Actors _outactors))

(event EventTick
  (params (DeltaSeconds :type Float%20%28single-precision%29)))

(event Input|KeyboardEvents|1
  (params (Key :type Key%20Structure :default "None"))
  (:Pressed
    (CallFunction|ChangePawn (Variables|Default|GetIndex))
    (bind _result (Math|Integer|IncrementInt (Variables|Default|GetIndex))
      (:%20%20
        (Variables|Default|SetIndex (Math|Integer|%(Integer) _result (Utilities|Array|Length (Variables|Default|GetOut%20Actors))))))))

(fn ConstructionScript)

(fn ChangePawn
  (params (Index :type Integer))
  (Pawn|UnPossess)
  (if (Utilities|Array|IsValidIndex (Variables|Default|GetOut%20Actors) Index)
    (Pawn|Possess (Utilities|Array|Get(acopy) (Variables|Default|GetOut%20Actors) (Variables|Default|GetIndex)))))